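; BP_BaseMonster is a monster Blueprint with melee attack, health and death logic, using slime animation montages.
; A BP_BaseCharacter entering AttackZone becomes the target; after a short delay the monster plays its attack montage and launches the target opposite the monster's forward vector as knockback.
; AnyDamage reduces HP and, at zero or below, plays a sped-up death montage once, then destroys the actor.
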(event `self.AttackZone.OnComponentBeginOverlap`
  (params (OverlappedComponent :type "PrimitiveComponent Object Reference") (OtherActor :type "Actor Object Reference") (OtherComp :type "PrimitiveComponent Object Reference") (OtherBodyIndex :type Integer) (bFromSweep :type Boolean) (SweepResult :type "HitResult Structure (by ref)"))
  ; 몬스터 공격범위 닿으면 공격실행
  (bind _asbp_base_character (cast `/Game/Blueprints/Character/BP_BaseCharacter` OtherActor))
  (set `self.TargetPlayer` _asbp_base_character)
  (`KismetSystemLibrary.Delay` 0.5)
  (`self.PlayAnimMontage` "/Game/Animations/Montage/AM_SlimeAttack.AM_SlimeAttack")
  ; 플레이어 넉백 현상
  (`self.LaunchCharacter` (`self.TargetPlayer`) (* (`self.GetActorForwardVector`) -800.0) false false))

(event `self.ReceiveAnyDamage`
  (params (Damage :type "Float (single-precision)") (DamageType :type "DamageType Object Reference") (InstigatedBy :type "Controller Object Reference") (DamageCauser :type "Actor Object Reference"))
  (bind _output_get (set `self.HP` (- (`self.HP`) Damage)))
  (if (<= _output_get 0.0)
    (`/Engine/EditorBlueprintResources/StandardMacros.DoOnce` false
      (:`Completed`
        (`self.PlayAnimMontage` "/Game/Animations/Montage/AM_SlimeDead.AM_SlimeDead" 3.0)
        (`KismetSystemLibrary.Delay` 0.2)
        (`self.K2_DestroyActor`)))))

(fn `UserConstructionScript`)